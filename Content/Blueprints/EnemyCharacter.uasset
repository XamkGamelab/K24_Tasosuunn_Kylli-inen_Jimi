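; EnemyCharacter is a twin-stick game enemy that repeatedly damages the hero while overlapping it.
; Overlap begin and end start and clear a looping timer that applies damage at the attack rate.
; AffectHealth recalculates health and, on death, adds score, ignores pawn and world-dynamic collision, detaches its controller, then explodes and is destroyed after a delay.
; Construction creates a dynamic mesh material instance.
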(event Custom|DamageTheHero
  (Default|AffectHealth (Variables|Default|GetHero) (Variables|Default|GetDamage)))

(event EventBeginPlay)

(event Collision|EventActorBeginOverlap
  (params (OtherActor :type Actor%20Object%20Reference))
  (bind _ashero_character (Utilities|Casting|CastToHeroCharacter OtherActor))
  (Variables|Default|SetHero _ashero_character)
  (Utilities|Time|SetTimerbyFunctionName 0 "DamageTheHero" (/ 1.0 (Variables|Default|GetAttackPerSecond)) true))

(event EventTick
  (params (DeltaSeconds :type Float%20%28single-precision%29)))

(event EventAffectHealth
  (params (Delta :type Float%20%28double-precision%29))
  (bind _capsulecomponent (Variables|Default|GetCapsuleComponent))
  (Class|BaseCharacter|CalculateHealth Delta)
  (if (Variables|Default|GetisDead)
    (bind _astwin_stick_mode (Utilities|Casting|CastToTwinStickMode (Game|GetGameMode)))
    (Default|IncrementScore _astwin_stick_mode (Variables|Default|GetDelta%20Score))
    (Collision|SetCollisionResponsetoChannel _capsulecomponent "ECC_WorldDynamic" "ECR_Ignore")
    (Collision|SetCollisionResponsetoChannel _capsulecomponent "ECC_Pawn" "ECR_Ignore")
    (Class|Pawn|DetachfromControllerPendingDestroy)
    (Utilities|FlowControl|Delay 3.0)
    (Game|SpawnActorfromClass "/Game/Blueprints/Explosion.Explosion_C" (Transformation|GetActorTransform) "Undefined" 0 0)
    (Actor|DestroyActor)))

(event Collision|EventActorEndOverlap
  (params (OtherActor :type Actor%20Object%20Reference))
  (if (== OtherActor (Variables|Default|GetHero))
    (Utilities|Time|ClearTimerbyFunctionName 0 "DamageTheHero")))

(fn ConstructionScript
  (bind _returnvalue (Rendering|Material|CreateDynamicMaterialInstance (Variables|Character|GetMesh) 0 0 "None" :!class /Script/Engine.PrimitiveComponent))
  (bind _output_get (Variables|Default|SetDynaMat _returnvalue))
  (Rendering|Material|SetVectorParameterValue :self _output_get :!class /Script/Engine.MaterialInstanceDynamic))